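; Base 2D flipbook player character for networked play, handling left/right movement and jumping.
; Axis input moves along the control rotation's forward vector and derives a movement state, which is sent to the server.
; OnRep_MovementState swaps PlayerInfo flipbooks and rotates the sprite to face the run direction, with no case for Fall.
; Jumping is allowed only when not falling, and its sound plays through a server-to-multicast event.
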(event `InputAxis|Move Left/Right`
  (params (AxisValue :type "Float (single-precision)"))
  ;[1 1 1] 角色移动
  (`self.AddMovementInput` (`KismetMathLibrary.GetForwardVector` (`self.GetControlRotation`)) AxisValue)
  (if (`NavMovementComponent.IsFalling` (`self.CharacterMovement`))
    (if (> (.z (`self.GetVelocity`)) 0.0)
      (`self.SetMovementState` "NewEnumerator2")
      (else
        (`self.SetMovementState` "NewEnumerator3")))
    (elif (== AxisValue 0.0)
      (`self.SetMovementState` "NewEnumerator0")
      (elif (> AxisValue 0.0)
        (`self.SetMovementState` "NewEnumerator1")
        (else
          (`self.SetMovementState` "NewEnumerator6"))))))

(event `self.SetMovementState`
  (params (MOvementState :type "/Game/Blueprints/Enums/EM_FB_MovementState Enum" :default "NewEnumerator0"))
  ;[1 1 1] 角色移动
  (`self.SRV_SetMovementState` MOvementState))

(event `SRV_SetMovementState`
  (params (MoveState :type "/Game/Blueprints/Enums/EM_FB_MovementState Enum" :default "NewEnumerator0"))
  ;[1 1 1] 角色移动
  (set `self.MovementState` MoveState))

(event `InputAction|Jump`
  (params (Key :type "Key Structure"))
  ;[1 1 1] 角色跳跃
  (:`Pressed`
    (if (not (`NavMovementComponent.IsFalling` (`self.CharacterMovement`)))
      (`self.Jump`)
      (`self.SRV_Jump` (`self.K2_GetActorLocation`) (`.JumpSFX_11_EF61E8F34B02E5166B9DD0B8F917704D` (break `/Game/Blueprints/Structures/MS_ST_PlayerInfo` (`self.PlayerInfo`)))))))

(event `MC_Jump`
  (params (Location :type "Vector Structure") (Sound :type "SoundBase Object Reference"))
  ;[1 1 1] 角色跳跃
  (`GameplayStatics.PlaySoundAtLocation` Sound Location (struct) 1.0 1.0 0.0 null null null null))

(event `SRV_Jump`
  (params (Location :type "Vector Structure") (Sound :type "SoundBase Object Reference"))
  ;[1 1 1] 角色跳跃
  (`self.MC_Jump` Location Sound))

(fn `GetPlayerRef`
  (returns (Player :type "/Game/Blueprints/Players/MS_FB_PlayerBase Object Reference"))
  (return self))

(fn `OnRep_MovementState`
  (bind (_idelanimation _runanimation _jumpanimation) (break `/Game/Blueprints/Structures/MS_ST_PlayerInfo` (`self.PlayerInfo`)))
  (switch `/Game/Blueprints/Enums/EM_FB_MovementState` (`self.MovementState`)
    (:`NewEnumerator0`
      (`PaperFlipbookComponent.SetFlipbook` (`self.Sprite`) _idelanimation))
    (:`NewEnumerator1`
      (`SceneComponent.K2_SetRelativeRotation` :`self` (`self.Sprite`))
      (`PaperFlipbookComponent.SetFlipbook` (`self.Sprite`) _runanimation))
    (:`NewEnumerator2`
      (`PaperFlipbookComponent.SetFlipbook` (`self.Sprite`) _jumpanimation))
    (:`NewEnumerator6`
      (`SceneComponent.K2_SetRelativeRotation` (`self.Sprite`) (struct :`Yaw` 180.0) false false)
      (`PaperFlipbookComponent.SetFlipbook` (`self.Sprite`) _runanimation))))

(fn `UserConstructionScript`
  (`parent.UserConstructionScript`))