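; Player character for a 2.5D three-lane auto-runner that shoots automatically and creates the player HUD on spawn.
; Looping timers drive constant forward movement along X and spawn scaled-down BP_Zidan projectiles, each destroyed after a short delay if it has not hit at spawn.
; Enhanced Input handles jumping and left/right lane switches, which use a clamped lane index, a timeline and lane Y positions to reposition the character.
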(event `self.ReceiveBeginPlay`
  ;[1 1 1] Enhance Input
  (bind _returnvalue (`|CreateWidget` "/Game/Assets/2_5D/UI/WUI_User_HUD.WUI_User_HUD_C"))
  (`UserWidget.AddToViewport` _returnvalue 0)
  (bind _asplayer_controller (cast `PlayerController` (`self.GetController`)))
  (bind _returnvalue_2 (pcsubsystem `EnhancedInputLocalPlayerSubsystem` _asplayer_controller))
  (`/Engine/EditorBlueprintResources/StandardMacros.IsValid` _returnvalue_2
    (:`Is Valid`
      (`EnhancedInputSubsystemInterface.AddMappingContext` _returnvalue_2 "/Game/Assets/2_5D/Inputs/IMC_2_5D_Default.IMC_2_5D_Default" 0 (struct))
      (`KismetSystemLibrary.K2_SetTimerDelegate` (delegate `MoveForward`) 0.01 true)
      (`KismetSystemLibrary.K2_SetTimerDelegate` (delegate `PerjectileZidan`) 0.2 true))))

(event `PerjectileZidan`
  (bind _returnvalue (`self.GetTransform`))
  (bind _returnvalue_2 (`|SpawnActorFromClass` "/Game/Assets/2_5D/Blueprints/BP_Zidan.BP_Zidan_C" (`KismetMathLibrary.MakeTransform` (`KismetMathLibrary.MakeVector` (+ (.x (.location _returnvalue)) 10.0) (.y (.location _returnvalue)) (- (.z (.location _returnvalue)) 10.0)) (.rotation _returnvalue) (0.3 0.3 0.3)) "Undefined" "OverrideRootScale" null null))
  (if (not (`/Game/Assets/2_5D/Blueprints/BP_Zidan.IsHit` _returnvalue_2))
    (`KismetSystemLibrary.Delay` 0.5)
    (if (`KismetSystemLibrary.IsValid` _returnvalue_2)
      (`self.K2_DestroyActor` _returnvalue_2))))

(event `MoveForward`
  (`self.AddMovementInput` (1.0 0.0 0.0) (`self.MoveValue`)))

(event `EnhancedInput|/Game/Assets/2_5D/Inputs/Actions/IA_2_5_D_MoveRight`
  (params (ActionValue :type "Float (double-precision)") (ElapsedSeconds :type "Float (double-precision)") (TriggeredSeconds :type "Float (double-precision)") (InputAction :type "InputAction Object Reference" :default "/Game/Assets/2_5D/Inputs/Actions/IA_2_5_D_MoveRight.IA_2_5_D_MoveRight"))
  (bind (_returnvalue_x _returnvalue_y _returnvalue_z) (`KismetMathLibrary.BreakVector` (`SceneComponent.K2_GetComponentLocation` (`self.CapsuleComponent`))))
  ;[1 1 1] 左右移动切换跑道
  (:`Triggered`
    (if (> ActionValue 0.0)
      (set `self.NewRoadLine` (`KismetMathLibrary.Clamp` (+ (`self.RoadLine`) 1) 0 2))
      (bind (_direction _movelaney) (`Timeline|LerpTimeline` :!via `PlayFromStart` :!label _label)
        (:`Finished`
          (set `self.RoadLine` (`self.NewRoadLine`))
          (`self.K2_SetActorLocation` (`KismetMathLibrary.MakeVector` _returnvalue_x (`KismetMathLibrary.Lerp` (`|GetArrayItem` (`self.LaneY`) (`self.RoadLine`)) (`|GetArrayItem` (`self.LaneY`) (`self.NewRoadLine`)) _movelaney) _returnvalue_z))))
      (elif (< ActionValue 0.0)
        (set `self.NewRoadLine` (`KismetMathLibrary.Clamp` (- (`self.RoadLine`) 1) 0 2))
        (goto _label :!via `PlayFromStart`)))))

(event `EnhancedInput|/Game/Assets/2_5D/Inputs/Actions/IA_2_5D_Jump`
  (params (ActionValue :type Boolean) (ElapsedSeconds :type "Float (double-precision)") (TriggeredSeconds :type "Float (double-precision)") (InputAction :type "InputAction Object Reference" :default "/Game/Assets/2_5D/Inputs/Actions/IA_2_5D_Jump.IA_2_5D_Jump"))
  (:`Triggered`
    (if (not (`self.IsInAir`))
      (`self.Jump`)))
  (:`Completed`
    (`self.StopJumping`)))

(fn `IsCanJump`
  (params (IsInAir :type Boolean :default false))
  (return))

(fn `UserConstructionScript`)