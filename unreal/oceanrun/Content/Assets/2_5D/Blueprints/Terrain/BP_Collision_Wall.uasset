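; BP_Collision_Wall is a destructible wall for the 2.5D game that awards score when shot down.
; Its Cube hit event reacts only to BP_Zidan bullets, calling ApplyPointDamage on the hit result's actor and subtracting the returned damage from WallHealth, initialized at BeginPlay.
; When health would reach zero or below, it adds points to CurrentScore in BP_OR_MyGame2_5DMode and destroys itself.
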(event `self.ReceiveBeginPlay`
  (set `self.WallHealth` 200))

(event `self.Cube.OnComponentHit`
  (params (HitComponent :type "PrimitiveComponent Object Reference") (OtherActor :type "Actor Object Reference") (OtherComp :type "PrimitiveComponent Object Reference") (NormalImpulse :type "Vector Structure") (Hit :type "HitResult Structure (by ref)"))
  (bind (_bblockinghit _binitialoverlap _time _distance _location _impactpoint _normal _impactnormal _physmat _hitactor) (`GameplayStatics.BreakHitResult` Hit))
  (cast `/Game/Assets/2_5D/Blueprints/BP_Zidan` OtherActor)
  (`KismetSystemLibrary.PrintString` "墙壁碰到子弹了")
  (bind _returnvalue (`GameplayStatics.ApplyPointDamage` _hitactor 10.0 _impactpoint Hit null null "/Script/Engine.DamageType"))
  (bind _returnvalue_2 (`KismetMathLibrary.FTrunc` (- (`self.WallHealth`) _returnvalue)))
  (if (> _returnvalue_2 0)
    (set `self.WallHealth` _returnvalue_2)
    (else
      (bind _asbp_or_my_game_2_5dmode (cast `/Game/Assets/2_5D/BP_OR_MyGame2_5DMode` (`GameplayStatics.GetGameMode`)))
      (set `/Game/Assets/2_5D/BP_OR_MyGame2_5DMode.CurrentScore` (+ (`/Game/Assets/2_5D/BP_OR_MyGame2_5DMode.CurrentScore` _asbp_or_my_game_2_5dmode) 200) _asbp_or_my_game_2_5dmode)
      (`self.K2_DestroyActor`))))

(fn `UserConstructionScript`)