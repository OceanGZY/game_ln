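; Endless-runner terrain tile for the 2.5D mode that populates itself with obstacles and triggers the next tile.
; On BeginPlay, SpawnCollision rolls a coin flip for a chicken at each of three road points and for a scaled wall.
; When the player overlaps SpawnBoxNewTile, the game mode spawns the next tile and adds multiplied score, player walk speed rises within a clamp, and the tile destroys itself after a delay.
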(event `self.ReceiveBeginPlay`
  (`self.SpawnCollision`))

(event `self.SpawnBoxNewTile.OnComponentBeginOverlap`
  (params (OverlappedComponent :type "PrimitiveComponent Object Reference") (OtherActor :type "Actor Object Reference") (OtherComp :type "PrimitiveComponent Object Reference") (OtherBodyIndex :type Integer) (bFromSweep :type Boolean) (SweepResult :type "HitResult Structure (by ref)"))
  (cast `/Game/Assets/2_5D/Blueprints/Player/BP_OR_2_5D_PlayerCharacter` OtherActor)
  (bind _asbp_or_my_game_2_5dmode (cast `/Game/Assets/2_5D/BP_OR_MyGame2_5DMode` (`GameplayStatics.GetGameMode`)))
  (`/Game/Assets/2_5D/BP_OR_MyGame2_5DMode.SpawnTile` _asbp_or_my_game_2_5dmode (`/Game/Assets/2_5D/BP_OR_MyGame2_5DMode.NextPos` _asbp_or_my_game_2_5dmode))
  (bind _asbp_or_my_game_2_5dmode_2 (cast `/Game/Assets/2_5D/BP_OR_MyGame2_5DMode` (`GameplayStatics.GetGameMode`)))
  (bind _output_get (set `/Game/Assets/2_5D/BP_OR_MyGame2_5DMode.CurrentScore` (+ (`/Game/Assets/2_5D/BP_OR_MyGame2_5DMode.CurrentScore` _asbp_or_my_game_2_5dmode_2) (* (`/Game/Assets/2_5D/BP_OR_MyGame2_5DMode.ScoreMutilple` _asbp_or_my_game_2_5dmode_2) 1)) _asbp_or_my_game_2_5dmode_2))
  (`KismetSystemLibrary.PrintString` (`KismetStringLibrary.Conv_IntToString` _output_get))
  (bind _asbp_or_2_5d_player_character (cast `/Game/Assets/2_5D/Blueprints/Player/BP_OR_2_5D_PlayerCharacter` (`GameplayStatics.GetPlayerCharacter` 0)))
  (bind _charactermovement (`Character.CharacterMovement` _asbp_or_2_5d_player_character))
  (set `CharacterMovementComponent.MaxWalkSpeed` (`KismetMathLibrary.FClamp` (* (`CharacterMovementComponent.MaxWalkSpeed` _charactermovement) 1.01) 600.0 1200.0) _charactermovement)
  (`KismetSystemLibrary.Delay` 20.0)
  (`self.K2_DestroyActor`))

(fn `SpawnCollision`
  (bind (_returnvalue_x _returnvalue_y) (`KismetMathLibrary.BreakVector` (`SceneComponent.K2_GetComponentLocation` (`self.Wall`))))
  (bind (_returnvalue_x_2 _returnvalue_y_2) (`KismetMathLibrary.BreakVector` (`SceneComponent.K2_GetComponentLocation` (`self.Road0`))))
  (bind (_returnvalue_x_3 _returnvalue_y_3) (`KismetMathLibrary.BreakVector` (`SceneComponent.K2_GetComponentLocation` (`self.Road1`))))
  (bind (_returnvalue_x_4 _returnvalue_y_4) (`KismetMathLibrary.BreakVector` (`SceneComponent.K2_GetComponentLocation` (`self.Road2`))))
  (`|ExecutionSequence`
    (:`then_0`
      (switch `int` (`KismetMathLibrary.RandomIntegerInRange` 0 1)
        (:`1`
          (`|SpawnActorFromClass` "/Game/Assets/2_5D/Blueprints/Terrain/Chicken/BP_CollisionChicken.BP_CollisionChicken_C" (`KismetMathLibrary.MakeTransform` (`KismetMathLibrary.MakeVector` _returnvalue_x_2 _returnvalue_y_2)) "Undefined" "OverrideRootScale" null null))))
    (:`then_1`
      (switch `int` (`KismetMathLibrary.RandomIntegerInRange` 0 1)
        (:`1`
          (`|SpawnActorFromClass` "/Game/Assets/2_5D/Blueprints/Terrain/Chicken/BP_CollisionChicken.BP_CollisionChicken_C" (`KismetMathLibrary.MakeTransform` (`KismetMathLibrary.MakeVector` _returnvalue_x_3 _returnvalue_y_3)) "Undefined" "OverrideRootScale" null null))))
    (:`then_2`
      (switch `int` (`KismetMathLibrary.RandomIntegerInRange` 0 1)
        (:`1`
          (`|SpawnActorFromClass` "/Game/Assets/2_5D/Blueprints/Terrain/Chicken/BP_CollisionChicken.BP_CollisionChicken_C" (`KismetMathLibrary.MakeTransform` (`KismetMathLibrary.MakeVector` _returnvalue_x_4 _returnvalue_y_4)) "Undefined" "OverrideRootScale" null null))))
    (:`then_3`
      (switch `int` (`KismetMathLibrary.RandomIntegerInRange` 0 1)
        (:`1`
          (`|SpawnActorFromClass` "/Game/Assets/2_5D/Blueprints/Terrain/BP_Collision_Wall.BP_Collision_Wall_C" (`KismetMathLibrary.MakeTransform` (`KismetMathLibrary.MakeVector` _returnvalue_x _returnvalue_y) (struct) (0.2 7.0 2.5)) "Undefined" "OverrideRootScale" null null))))))

(fn `UserConstructionScript`)