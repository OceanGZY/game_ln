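; A destructible chicken target in a 2.5D game that loses health when hit by BP_Zidan bullets and awards score when killed.
; On hit, it applies point damage to the hit actor and subtracts the returned amount from its own health.
; A dynamic material on HealthBar, created in the construction script, receives H_Percent from an integer division of health.
; At zero health, it adds to the game mode's score and destroys itself.
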(event `self.ReceiveBeginPlay`
  (set `self.ChickenHealth` 100))

(event `self.Chicken.OnComponentHit`
  (params (HitComponent :type "PrimitiveComponent Object Reference") (OtherActor :type "Actor Object Reference") (OtherComp :type "PrimitiveComponent Object Reference") (NormalImpulse :type "Vector Structure") (Hit :type "HitResult Structure (by ref)"))
  (bind (_bblockinghit _binitialoverlap _time _distance _location _impactpoint _normal _impactnormal _physmat _hitactor) (`GameplayStatics.BreakHitResult` Hit))
  (cast `/Game/Assets/2_5D/Blueprints/BP_Zidan` OtherActor)
  (`KismetSystemLibrary.PrintString` "小鸡碰撞子弹啦")
  (bind _returnvalue (`GameplayStatics.ApplyPointDamage` _hitactor 10.0 _impactpoint Hit null null "/Script/Engine.DamageType"))
  (bind _returnvalue_2 (`KismetMathLibrary.FTrunc` (- (`self.ChickenHealth`) _returnvalue)))
  (if (> _returnvalue_2 0)
    (bind _output_get (set `self.ChickenHealth` _returnvalue_2))
    (`KismetSystemLibrary.PrintString` "剩余血量")
    (`KismetSystemLibrary.PrintString` (`KismetStringLibrary.Conv_IntToString` _output_get))
    (`MaterialInstanceDynamic.SetScalarParameterValue` (`self.MTR_Health`) "H_Percent" (`KismetMathLibrary.Conv_IntToDouble` (/ _output_get 100)))
    (else
      (`MaterialInstanceDynamic.SetScalarParameterValue` (`self.MTR_Health`) "H_Percent" 0.01)
      (bind _asbp_or_my_game_2_5dmode (cast `/Game/Assets/2_5D/BP_OR_MyGame2_5DMode` (`GameplayStatics.GetGameMode`)))
      (set `/Game/Assets/2_5D/BP_OR_MyGame2_5DMode.CurrentScore` (+ (`/Game/Assets/2_5D/BP_OR_MyGame2_5DMode.CurrentScore` _asbp_or_my_game_2_5dmode) 100) _asbp_or_my_game_2_5dmode)
      (`self.K2_DestroyActor`))))

(fn `UserConstructionScript`
  (bind _returnvalue (`PrimitiveComponent.CreateDynamicMaterialInstance` (`self.HealthBar`) 0 null "None"))
  (set `self.MTR_Health` _returnvalue))