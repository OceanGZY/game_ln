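; Player character Blueprint for 2D play, handling horizontal movement and jumping through Enhanced Input.
; BeginPlay adds the 2D default mapping context to the owning player controller's input subsystem.
; The move action scales movement along the fixed world X axis, independent of actor or camera rotation.
; The jump action calls Jump when triggered and StopJumping when completed.
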(event `self.ReceiveBeginPlay`
  ;[1 1 1] Enhance Input
  (bind _asplayer_controller (cast `PlayerController` (`self.GetController`)))
  (bind _returnvalue (pcsubsystem `EnhancedInputLocalPlayerSubsystem` _asplayer_controller))
  (`/Engine/EditorBlueprintResources/StandardMacros.IsValid` _returnvalue
    (:`Is Valid`
      (`EnhancedInputSubsystemInterface.AddMappingContext` _returnvalue "/Game/Assets/2D/Inputs/IMC_2D_Default.IMC_2D_Default" 0 (struct)))))

(event `EnhancedInput|/Game/Assets/2D/Inputs/Actions/IA_2D_Move`
  (params (ActionValue :type "Float (double-precision)") (ElapsedSeconds :type "Float (double-precision)") (TriggeredSeconds :type "Float (double-precision)") (InputAction :type "InputAction Object Reference" :default "/Game/Assets/2D/Inputs/Actions/IA_2D_Move.IA_2D_Move"))
  (:`Triggered`
    (`self.AddMovementInput` (`KismetMathLibrary.GetForwardVector` (struct)) ActionValue)))

(event `EnhancedInput|/Game/Assets/2D/Inputs/Actions/IA_2D_Jump`
  (params (ActionValue :type Boolean) (ElapsedSeconds :type "Float (double-precision)") (TriggeredSeconds :type "Float (double-precision)") (InputAction :type "InputAction Object Reference" :default "/Game/Assets/2D/Inputs/Actions/IA_2D_Jump.IA_2D_Jump"))
  (:`Triggered`
    (`self.Jump`))
  (:`Completed`
    (`self.StopJumping`)))

(fn `UserConstructionScript`)