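; BP_Banzi is a self-chaining, score-carrying segment for a 2D game that shows its Score on a text render.
; When the player character overlaps Box, it spawns the next BP_Banzi at ArrowEnd with an increased Score, shows that new value, then destroys itself after a delay.
; Overlapping DeadBox reloads the current level after a short pause, restarting the run.
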(event `self.ReceiveBeginPlay`
  (`TextRenderComponent.K2_SetText` (`self.TextRender`) (`KismetTextLibrary.Conv_IntToText` (`self.Score`) false true 2)))

(event `self.Box.OnComponentBeginOverlap`
  (params (OverlappedComponent :type "PrimitiveComponent Object Reference") (OtherActor :type "Actor Object Reference") (OtherComp :type "PrimitiveComponent Object Reference") (OtherBodyIndex :type Integer) (bFromSweep :type Boolean) (SweepResult :type "HitResult Structure (by ref)"))
  (cast `/Game/Assets/2D/Blueprints/Player/BP_OR_2D_PlayerCharacter` OtherActor)
  (bind _returnvalue (`|SpawnActorFromClass` "BP_Banzi_C" (`SceneComponent.K2_GetComponentToWorld` (`self.ArrowEnd`)) "Undefined" "OverrideRootScale" null null))
  (bind _output_get (set `/Game/Assets/2D/Blueprints/BP_Banzi.Score` (+ (`self.Score`) 10) _returnvalue))
  (`TextRenderComponent.K2_SetText` (`self.TextRender`) (`KismetTextLibrary.Conv_IntToText` _output_get))
  (`KismetSystemLibrary.Delay` 20.0)
  (`self.K2_DestroyActor`))

(event `self.DeadBox.OnComponentBeginOverlap`
  (params (OverlappedComponent :type "PrimitiveComponent Object Reference") (OtherActor :type "Actor Object Reference") (OtherComp :type "PrimitiveComponent Object Reference") (OtherBodyIndex :type Integer) (bFromSweep :type Boolean) (SweepResult :type "HitResult Structure (by ref)"))
  (cast `/Game/Assets/2D/Blueprints/Player/BP_OR_2D_PlayerCharacter` OtherActor)
  (`KismetSystemLibrary.Delay` 0.5)
  (bind _returnvalue (`GameplayStatics.GetCurrentLevelName` true))
  (`GameplayStatics.OpenLevel` (`KismetStringLibrary.Conv_StringToName` _returnvalue)))

(fn `UserConstructionScript`)