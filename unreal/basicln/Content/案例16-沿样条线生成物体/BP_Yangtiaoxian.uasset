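; BP_Yangtiaoxian is a spline-based placement actor that lays cone static meshes along its Spline component.
; The construction script divides the spline length by SpawnNum and adds a static mesh component at each evenly spaced distance.
; Each cone takes the spline's local rotation, and its world-space spline location is converted to actor-relative space with InverseTransformLocation.
; The event graph has no active logic.
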(fn `UserConstructionScript`
  (bind _spline (`self.Spline`))
  (for _index (range (+ (`self.SpawnNum`) 1))
    (bind _returnvalue (`KismetMathLibrary.Conv_IntToDouble` (* _index (/ (`SplineComponent.GetSplineLength` (`self.Spline`)) (`self.SpawnNum`)))))
    (bind _returnvalue_2 (`AddComponent|NODE_AddStaticMeshComponent-0` :`RelativeTransform` (`KismetMathLibrary.MakeTransform` (`KismetMathLibrary.InverseTransformLocation` (`self.GetTransform`) (`SplineComponent.GetLocationAtDistanceAlongSpline` _spline _returnvalue "World")) (`SplineComponent.GetRotationAtDistanceAlongSpline` _spline _returnvalue "Local"))))
    (`StaticMeshComponent.SetStaticMesh` _returnvalue_2 "/Game/StarterContent/Shapes/Shape_Cone.Shape_Cone")))