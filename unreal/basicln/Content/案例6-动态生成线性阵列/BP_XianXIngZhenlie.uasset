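; Actor Blueprint that procedurally builds a linear array of static meshes along its local X axis.
; The Construction Script loops from zero to SpawnNum, adding a mesh component at each multiple of SpawnDis and assigning the Stat mesh.
; BeginPlay only prints a fixed run of loop indices, unrelated to the array.
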(event `self.ReceiveBeginPlay`
  (for _index (range 7)
    (`KismetSystemLibrary.PrintString` (`KismetStringLibrary.Conv_IntToString` _index))))

(fn `UserConstructionScript`
  (for _index (range (+ (`self.SpawnNum`) 1))
    (bind _returnvalue (`AddComponent|NODE_AddStaticMeshComponent-0` :`RelativeTransform` (`KismetMathLibrary.MakeTransform` (`KismetMathLibrary.MakeVector` (* _index (`self.SpawnDis`))))))
    (`StaticMeshComponent.SetStaticMesh` _returnvalue (`self.Stat`))))