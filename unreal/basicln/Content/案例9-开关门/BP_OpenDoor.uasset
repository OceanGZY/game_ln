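; BP_OpenDoor is a swinging door that opens when any actor overlaps its Box and closes when an overlap ends.
; The overlapping actor's side along world X selects a positive or negative quarter-turn yaw, played by the OpenDoor timeline.
; The CloseDoor timeline returns yaw to zero.
; Each timeline stops the other and lerps from the door's current yaw, so reversals start mid-swing.
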(event `self.Box.OnComponentBeginOverlap`
  (params (OverlappedComponent :type "PrimitiveComponent Object Reference") (OtherActor :type "Actor Object Reference") (OtherComp :type "PrimitiveComponent Object Reference") (OtherBodyIndex :type Integer) (bFromSweep :type Boolean) (SweepResult :type "HitResult Structure (by ref)"))
  (bind _door (`self.Door`))
  (bind _returnvalue_x (`KismetMathLibrary.BreakVector` (- (`self.K2_GetActorLocation`) (`self.K2_GetActorLocation` OtherActor))))
  (bind (_relativerotation_roll _relativerotation_pitch _relativerotation_yaw) (`KismetMathLibrary.BreakRotator` (`SceneComponent.RelativeRotation` _door)))
  (`TimelineComponent.Stop` (`self.CloseDoor`))
  (set `self.Dir` (> _returnvalue_x 0.0))
  (bind (_direction _value) (`Timeline|OpenDoor` :!via `PlayFromStart`)
    (:`Update`
      (`SceneComponent.K2_SetRelativeRotation` _door (`KismetMathLibrary.MakeRotator` 0.0 0.0 (`KismetMathLibrary.Lerp` _relativerotation_yaw (`KismetMathLibrary.SelectFloat` 90.0 -90.0 (`self.Dir`)) _value)) false false))))

(event `self.Box.OnComponentEndOverlap`
  (params (OverlappedComponent :type "PrimitiveComponent Object Reference") (OtherActor :type "Actor Object Reference") (OtherComp :type "PrimitiveComponent Object Reference") (OtherBodyIndex :type Integer))
  (bind _door (`self.Door`))
  (bind (_relativerotation_roll _relativerotation_pitch _relativerotation_yaw) (`KismetMathLibrary.BreakRotator` (`SceneComponent.RelativeRotation` _door)))
  (`TimelineComponent.Stop` (`self.OpenDoor`))
  (bind (_direction _value) (`Timeline|CloseDoor` :!via `PlayFromStart`)
    (:`Update`
      (`SceneComponent.K2_SetRelativeRotation` _door (`KismetMathLibrary.MakeRotator` 0.0 0.0 (`KismetMathLibrary.Lerp` _relativerotation_yaw 0.0 _value)) false false))))

(fn `UserConstructionScript`)