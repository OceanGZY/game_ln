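; Key-controlled elevator that lifts a cube platform up and down while the player toggles it from a trigger area.
; Overlapping ElevatorKey shows a prompt widget and enables control; leaving hides it and disables control.
; FControllElevato toggles between stopping and resuming a Timeline, using the saved direction to play from start or reverse.
; The Timeline drives the cube's relative Z and loops back and forth with a short pause at each end.
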(event `FControllElevato`
  (bind (_relativelocation_x _relativelocation_y) (`KismetMathLibrary.BreakVector` (`SceneComponent.RelativeLocation` (`self.Cube`))))
  (if (`self.bCancontrol`)
    (if (`self.bIsStop`)
      (set `self.bIsStop` false)
      (switch `ETimelineDirection` (`self.tlDir`)
        (:`Forward`
          (bind (_direction _value) (`Timeline|Timeline` :!via `PlayFromStart` :!label _label)
            (:`Update`
              (set `self.tlDir` _direction)
              (`SceneComponent.K2_SetRelativeLocation` (`self.Cube`) (`KismetMathLibrary.MakeVector` _relativelocation_x _relativelocation_y (* _value 500.0)) false false))
            (:`Finished`
              (if (`|EnumEquality` _direction "Forward")
                (`KismetSystemLibrary.Delay` 1.0)
                (goto _label :!via `Reverse`)
                (else
                  (`KismetSystemLibrary.Delay` 1.0)
                  (goto _label :!via `PlayFromStart`))))))
        (:`Backward`
          (goto _label :!via `Reverse`)))
      (else
        (set `self.bIsStop` true)
        (goto _label :!via `Stop`)))))

(event `self.ElevatorKey.OnComponentBeginOverlap`
  (params (OverlappedComponent :type "PrimitiveComponent Object Reference") (OtherActor :type "Actor Object Reference") (OtherComp :type "PrimitiveComponent Object Reference") (OtherBodyIndex :type Integer) (bFromSweep :type Boolean) (SweepResult :type "HitResult Structure (by ref)"))
  (`KismetSystemLibrary.PrintString` (`KismetSystemLibrary.GetDisplayName` OtherComp))
  (`SceneComponent.SetVisibility` (`self.Widget`) true false)
  (set `self.bCancontrol` true))

(event `self.ReceiveBeginPlay`
  (`SceneComponent.SetVisibility` (`self.Widget`) false false))

(event `self.ElevatorKey.OnComponentEndOverlap`
  (params (OverlappedComponent :type "PrimitiveComponent Object Reference") (OtherActor :type "Actor Object Reference") (OtherComp :type "PrimitiveComponent Object Reference") (OtherBodyIndex :type Integer))
  (`SceneComponent.SetVisibility` (`self.Widget`) false false)
  (set `self.bCancontrol` false))

(fn `UserConstructionScript`)