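; BP_JUxingZhenlie is an actor that generates a flat rectangular array of copies of one configurable static mesh.
; Its Construction Script runs nested loops from zero to the horizontal and vertical counts, adding a Static Mesh Component per cell.
; Each relative location is loop index times spacing, with vertical along X and horizontal along Y.
; The Event Graph holds only disabled placeholder events, so nothing runs there.
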(fn `UserConstructionScript`
  (for _index (range (+ (`self.HorizontalNum`) 1))
    (for _index_2 (range (+ (`self.VerticalNum`) 1))
      (bind _returnvalue (`AddComponent|NODE_AddStaticMeshComponent-0` :`RelativeTransform` (`KismetMathLibrary.MakeTransform` (`KismetMathLibrary.MakeVector` (* _index_2 (`self.VerticalDis`)) (* _index (`self.HorizontalDis`))))))
      (`StaticMeshComponent.SetStaticMesh` _returnvalue (`self.StaticMeshhhh`)))))