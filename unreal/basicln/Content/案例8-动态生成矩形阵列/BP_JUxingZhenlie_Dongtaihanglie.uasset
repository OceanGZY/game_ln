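; Example actor that builds a rectangular array of static mesh components from a total count, row and column limits and spacing variables.
; The Construction Script runs nested loops, filling rows along X and stepping along Y.
; A remaining-count variable caps each row, so the last may be partial, and generation stops at the total or the grid limit.
; Each placement prints the remaining count; EventGraph is unused.
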(fn `UserConstructionScript`
  (set `self.Nnunm` (`self.AllCount`))
  (for _index (range 1 (+ (`self.HorizontalNum`) 1))
    (if (< (`self.VerticalNum`) (`self.Nnunm`))
      (set `self.EveryHorizontalNum` (`self.VerticalNum`))
      (else
        (set `self.EveryHorizontalNum` (`self.Nnunm`))))
    (for _index_2 (range 1 (+ (`self.EveryHorizontalNum`) 1))
      (bind _returnvalue (`AddComponent|NODE_AddStaticMeshComponent-0` :`RelativeTransform` (`KismetMathLibrary.MakeTransform` (`KismetMathLibrary.MakeVector` (* _index_2 (`self.VerticalDis`)) (* _index (`self.HorizontalDis`))))))
      (`StaticMeshComponent.SetStaticMesh` _returnvalue (`self.StaticMeshhhh`))
      (`/Engine/EditorBlueprintResources/StandardMacros.DecrementInt` (`self.Nnunm`)
        (:`  `
          (`KismetSystemLibrary.PrintString` (`KismetStringLibrary.Conv_IntToString` (`self.Nnunm`))))))))