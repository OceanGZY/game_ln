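; Actor Blueprint that procedurally builds a ring array of static meshes around its origin.
; The Construction Script loops from 0 to SpawnNum, adding a StaticMeshComponent per index and assigning it the StaticMeshhh mesh.
; Each component's location comes from rotating a Radius-length X vector by an evenly stepped yaw, which also sets its rotation to face outward along X.
; The Event Graph holds no active logic.
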(fn `UserConstructionScript`
  (for _index (range (+ (`self.SpawnNum`) 1))
    (bind _returnvalue (`KismetMathLibrary.MakeRotator` 0.0 0.0 (* _index (/ 360 (`self.SpawnNum`)))))
    (bind _returnvalue_2 (`AddComponent|NODE_AddStaticMeshComponent-0` :`RelativeTransform` (`KismetMathLibrary.MakeTransform` (`KismetMathLibrary.GreaterGreater_VectorRotator` (`KismetMathLibrary.MakeVector` (`self.Radius`)) _returnvalue) _returnvalue)))
    (`StaticMeshComponent.SetStaticMesh` _returnvalue_2 (`self.StaticMeshhh`))))