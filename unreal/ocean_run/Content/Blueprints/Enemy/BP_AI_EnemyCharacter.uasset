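; Enemy AI character that periodically issues movement toward the player's BP_OR_GunMan pawn.
; AiMove runs at BeginPlay and on a looping timer whose interval of a few seconds is randomized once.
; It passes both a random nearby reachable point and the player as target to AIMoveTo, so the target actor takes precedence.
; Incoming damage is only printed for debugging, with no health handling.
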(event `self.ReceiveBeginPlay`
  (`self.AiMove`)
  (`KismetSystemLibrary.K2_SetTimerDelegate` (delegate `AiMove`) (`KismetMathLibrary.RandomFloatInRange` 3.0 5.0) true))

(event `AiMove`
  (bind _asbp_or_gun_man (cast `/Game/Blueprints/Player/GunMan/BP_OR_GunMan` (`GameplayStatics.GetPlayerPawn` 0)))
  (`|AIMoveTo` self (`NavigationSystemV1.K2_GetRandomReachablePointInRadius` (`self.K2_GetActorLocation`) 500.0 null null) _asbp_or_gun_man))

(event `self.ReceiveAnyDamage`
  (params (Damage :type "Float (single-precision)") (DamageType :type "DamageType Object Reference") (InstigatedBy :type "Controller Object Reference") (DamageCauser :type "Actor Object Reference"))
  (`KismetSystemLibrary.PrintString` "被打中了，伤害值是")
  (`KismetSystemLibrary.PrintString` (`KismetStringLibrary.Conv_DoubleToString` Damage)))

(fn `UserConstructionScript`)