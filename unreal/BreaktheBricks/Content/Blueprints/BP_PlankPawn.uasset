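; BP_PlankPawn is the player's paddle pawn, which slides under touch control and ends the game when a ball reaches its trigger.
; It adds an Enhanced Input mapping context on BeginPlay, and the touch action sets a flag that Tick reads.
; While touched, a trace under the finger drives the plank's world X, keeping Y and fixing Z.
; A BP_Ball overlapping the Trigger component shows the game-over widget.
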(event `self.ReceiveBeginPlay`
  (bind _returnvalue (pcsubsystem `EnhancedInputLocalPlayerSubsystem` (`GameplayStatics.GetPlayerController` 0)))
  ;[1 1 1] 配置 增强输入
  (`/Engine/EditorBlueprintResources/StandardMacros.IsValid` _returnvalue
    (:`Is Valid`
      (`EnhancedInputSubsystemInterface.AddMappingContext` _returnvalue "/Game/Inputs/IMC_Action.IMC_Action" 0 (struct)))))

(event `EnhancedInput|/Game/Inputs/IA_TouchInput`
  (params (ActionValue :type Boolean) (ElapsedSeconds :type "Float (double-precision)") (TriggeredSeconds :type "Float (double-precision)") (InputAction :type "InputAction Object Reference" :default "/Game/Inputs/IA_TouchInput.IA_TouchInput"))
  (:`Triggered`
    (set `self.IsTouch` true))
  (:`Completed`
    (set `self.IsTouch` false)))

(event `self.ReceiveTick`
  (params (DeltaSeconds :type "Float (single-precision)"))
  (bind _playerplank (`self.PlayerPlank`))
  (bind _playerplank_2 (`self.PlayerPlank`))
  (bind (_returnvalue_x _returnvalue_y) (`KismetMathLibrary.BreakVector` (`SceneComponent.K2_GetComponentLocation` _playerplank_2)))
  (if (`self.IsTouch`)
    (`SceneComponent.K2_SetWorldLocation` _playerplank_2 (`KismetMathLibrary.MakeVector` (.x (`.Location` (`GameplayStatics.BreakHitResult` (`PlayerController.GetHitResultUnderFingerByChannel` (`GameplayStatics.GetPlayerController` 0) "Touch1" "TraceTypeQuery1" true)))) _returnvalue_y 100.0) false false)
    (else
      (`SceneComponent.K2_SetWorldLocation` _playerplank (`SceneComponent.K2_GetComponentLocation` _playerplank) false false))))

(event `self.Trigger.OnComponentBeginOverlap`
  (params (OverlappedComponent :type "PrimitiveComponent Object Reference") (OtherActor :type "Actor Object Reference") (OtherComp :type "PrimitiveComponent Object Reference") (OtherBodyIndex :type Integer) (bFromSweep :type Boolean) (SweepResult :type "HitResult Structure (by ref)"))
  (cast `/Game/Blueprints/BP_Ball` OtherActor)
  (bind _returnvalue (`|CreateWidget` "/Game/WUI_GameOver.WUI_GameOver_C"))
  (`UserWidget.AddToViewport` _returnvalue 0))

(fn `UserConstructionScript`)