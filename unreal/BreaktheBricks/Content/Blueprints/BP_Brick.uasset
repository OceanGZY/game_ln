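; BP_Brick is a breakable brick that takes two hits from BP_Ball to destroy.
; On BeginPlay it sets its world height, then listens for the ball overlapping its Box component.
; The first hit swaps the material, spawns an attached Niagara effect and plays a sound.
; The next hit spawns a second effect and sound at once, then destroys the actor after a short delay.
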(event `self.ReceiveBeginPlay`
  (bind _brick (`self.Brick`))
  (bind (_returnvalue_x _returnvalue_y) (`KismetMathLibrary.BreakVector` (`SceneComponent.K2_GetComponentLocation` _brick)))
  (`SceneComponent.K2_SetWorldLocation` _brick (`KismetMathLibrary.MakeVector` _returnvalue_x _returnvalue_y 100.0) false false))

(event `self.Box.OnComponentBeginOverlap`
  (params (OverlappedComponent :type "PrimitiveComponent Object Reference") (OtherActor :type "Actor Object Reference") (OtherComp :type "PrimitiveComponent Object Reference") (OtherBodyIndex :type Integer) (bFromSweep :type Boolean) (SweepResult :type "HitResult Structure (by ref)"))
  (bind _brick (`self.Brick`))
  (cast `/Game/Blueprints/BP_Ball` OtherActor)
  (if (`self.IsFirstCollision`)
    (`PrimitiveComponent.SetMaterial` _brick 0 "/Game/Matetials/MAT_Brick_2.MAT_Brick_2")
    (`|ExecutionSequence`
      (:`then_0`
        (`NiagaraFunctionLibrary.SpawnSystemAttached` "/Game/VisualEffects/NS_Brick.NS_Brick" _brick "None" (0.0 0.0 50.0) (struct) "KeepRelativeOffset")
        (`GameplayStatics.PlaySoundAtLocation` "/Game/Sounds/hit_01_Cue.hit_01_Cue" (0.0 0.0 0.0) (struct) 1.0 1.0 0.0 null null null null))
      (:`then_1`
        (set `self.IsFirstCollision` false)))
    (else
      (`|ExecutionSequence`
        (:`then_0`
          (`KismetSystemLibrary.Delay` 0.2)
          (`self.K2_DestroyActor`))
        (:`then_1`
          (`NiagaraFunctionLibrary.SpawnSystemAtLocation` "/Game/VisualEffects/NS_Brick_2.NS_Brick_2" (`SceneComponent.K2_GetComponentLocation` _brick))
          (`GameplayStatics.PlaySoundAtLocation` "/Game/Sounds/hit_02_Cue.hit_02_Cue" (0.0 0.0 0.0) (struct) 1.0 1.0 0.0 null null null null))))))

(fn `UserConstructionScript`)