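; BP_Enemy is an enemy ship Blueprint that randomizes its colors and animates its scale on spawn.
; Its SetColor event creates a dynamic instance of M_Base_Ship, setting random body and wing colors from separate four-color palettes, and applies it to the ship mesh.
; The same event then plays a timeline that drives the actor's uniform scale.
; BeginPlay, overlap, tick and construction logic are empty.
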(event `self.SetColor`
  (set `self.BodyColorIndex` (`KismetMathLibrary.RandomIntegerInRange` 0 3))
  (set `self.WingColorIndex` (`KismetMathLibrary.RandomIntegerInRange` 0 3))
  (bind _returnvalue (`KismetMaterialLibrary.CreateDynamicMaterialInstance` "/Game/SpaceshipBattle/Materials/M_Base_Ship.M_Base_Ship"))
  (`MaterialInstanceDynamic.SetVectorParameterValue` _returnvalue "Color1" (select `int` (`self.BodyColorIndex`) :`0` (struct :`R` 0.041559 :`G` 1.0 :`B` 0.080272 :`A` 1.0) :`1` (struct :`R` 0.006095 :`G` 0.056185 :`B` 1.0 :`A` 1.0) :`2` (struct :`R` 0.928061 :`B` 1.0 :`A` 1.0) :`3` (struct :`R` 1.0 :`G` 0.061336 :`B` 0.04144 :`A` 1.0) :!type "LinearColor Structure"))
  (`MaterialInstanceDynamic.SetVectorParameterValue` _returnvalue "Color2" (select `int` (`self.WingColorIndex`) :`0` (struct :`R` 1.0 :`G` 0.093803 :`B` 0.533589 :`A` 1.0) :`1` (struct :`R` 1.0 :`G` 0.188886 :`A` 1.0) :`2` (struct :`R` 0.140571 :`G` 0.369792 :`A` 1.0) :`3` (struct :`G` 0.316752 :`B` 1.0 :`A` 1.0) :!type "LinearColor Structure"))
  (`PrimitiveComponent.SetMaterial` (`self.ShipStaticMeshComp`) 0 _returnvalue)
  (bind (_direction _scale) (`Timeline|SpawnScaleTimeline`)
    (:`Update`
      (`self.SetActorScale3D` (`KismetMathLibrary.Conv_DoubleToVector` _scale)))))

(fn `UserConstructionScript`)