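; Player bird for a Flappy Bird-style game, driven by a Ready, Playing and Dead state.
; The jump input starts the game from Ready, enabling capsule physics, and during play zeroes velocity before applying an upward force.
; While Playing, SpawnPiple re-calls itself on a delay to keep spawning pipe actors.
; Any capsule hit sets Dead, and game start and game over are both broadcast through event dispatchers.
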(event `InputAction|FB_JUMP`
  (params (Key :type "Key Structure"))
  (:`Pressed`
    (switch `/Game/Blueprints/fb_state` (`self.State`)
      (:`NewEnumerator0`
        (`self.fb_startGame`))
      (:`NewEnumerator1`
        (`PrimitiveComponent.SetPhysicsLinearVelocity` (`self.Capsule`) (0.0 0.0 0.0) false "None")
        (`PrimitiveComponent.AddForce` (`self.Capsule`) (0.0 0.0 100000.0) "None" false)))))

(event `self.ReceiveBeginPlay`
  (`self.SpawnPiple`))

(event `SpawnPiple`
  (switch `/Game/Blueprints/fb_state` (`self.State`)
    (:`NewEnumerator1`
      (`|SpawnActorFromClass` "/Game/Blueprints/fb_guandao.fb_guandao_C" (`KismetMathLibrary.MakeTransform` (0.0 0.0 0.0)) "Undefined" "OverrideRootScale" null null)
      (`KismetSystemLibrary.Delay` 2.0)
      (`self.SpawnPiple`))))

(event `self.Capsule.OnComponentHit`
  (params (HitComponent :type "PrimitiveComponent Object Reference") (OtherActor :type "Actor Object Reference") (OtherComp :type "PrimitiveComponent Object Reference") (NormalImpulse :type "Vector Structure") (Hit :type "HitResult Structure (by ref)"))
  (`self.fb_gameOver`))

(fn `fb_gameOver`
  (`KismetSystemLibrary.PrintString` "撞到东西了")
  (set `self.State` "NewEnumerator2")
  (`self.ed_GameOver`))

(fn `fb_startGame`
  (set `self.State` "NewEnumerator1")
  (`PrimitiveComponent.SetSimulatePhysics` (`self.Capsule`) true)
  (`self.SpawnPiple`)
  (`self.ed_GameStart`))

(fn `UserConstructionScript`)