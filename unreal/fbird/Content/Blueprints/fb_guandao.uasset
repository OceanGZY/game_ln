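; fb_guandao is a moving obstacle actor for what appears to be a Flappy Bird-style game.
; On BeginPlay it sets its starting Y and a random height, takes a ten-second lifespan, and binds to the fb_bird pawn's game start and game over dispatchers.
; Tick moves it along +Y by a fixed, frame-rate-dependent step while Moving is set.
; Game start enables movement; game over stops it and destroys it after a short delay.
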(event `self.ReceiveBeginPlay`
  (`self.K2_SetActorLocation` (`KismetMathLibrary.MakeVector` 0.0 -240.0 (`KismetMathLibrary.RandomFloatInRange` 62.0 110.0)))
  (`self.SetLifeSpan` 10.0)
  (bind _asfb_bird (cast `/Game/Blueprints/fb_bird` (`GameplayStatics.GetPlayerPawn` 0)))
  (add `/Game/Blueprints/fb_bird.ed_GameStart` _asfb_bird (delegate `ed_GameStart_Event`))
  (add `/Game/Blueprints/fb_bird.ed_GameOver` _asfb_bird (delegate `ed_GameOver_Event`)))

(event `ed_GameOver_Event`
  (set `self.bMoving` false)
  (`KismetSystemLibrary.Delay` 2.0)
  (`self.K2_DestroyActor`))

(event `ed_GameStart_Event`
  (set `self.bMoving` true))

(event `self.ReceiveTick`
  (params (DeltaSeconds :type "Float (single-precision)"))
  (if (`self.bMoving`)
    (`self.K2_AddActorWorldOffset` (0.0 1.0 0.0))))

(fn `UserConstructionScript`)