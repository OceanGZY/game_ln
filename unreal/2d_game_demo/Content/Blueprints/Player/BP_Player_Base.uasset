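; Base Paper2D player character with side-to-side movement, jumping and a replicated movement state that drives its animation.
; Axis input moves along the control rotation's forward vector and, when grounded, picks idle or run states, which go through a server event.
; The state's RepNotify swaps PlayerInfo flipbooks, rotates the sprite for runs and plays the jump sound.
; The velocity-based Jump/Fall selection is unwired, so those states are never set here.
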(event `InputAxis|Move Right/Left`
  (params (AxisValue :type "Float (single-precision)"))
  (`self.AddMovementInput` (`KismetMathLibrary.GetForwardVector` (`self.GetControlRotation`)) AxisValue)
  (if (`NavMovementComponent.IsFalling` (`self.CharacterMovement`))
    _
    (elif (== AxisValue 0.0)
      (`self.SetMovementStates` "NewEnumerator1")
      (elif (> AxisValue 0.0)
        (`self.SetMovementStates` "NewEnumerator2")
        (else
          (`self.SetMovementStates` "NewEnumerator3"))))))

(event `InputAction|Jump`
  (params (Key :type "Key Structure"))
  (:`Pressed`
    (if (not (`NavMovementComponent.IsFalling` (`self.CharacterMovement`)))
      (`self.Jump`))))

(event `SetMovementStates`
  (params (MovementStates :type "/Game/Blueprints/Enums/E_MovementStates Enum" :default "NewEnumerator1"))
  (`self.SRV_SetMovementStates` MovementStates))

(event `SRV_SetMovementStates`
  (params (MovementStates :type "/Game/Blueprints/Enums/E_MovementStates Enum" :default "NewEnumerator1"))
  (set `self.MovementStates` MovementStates))

(fn `OnRep_MovementStates`
  (bind (_idleanimation _runanimation _jumpanimation _fallanimation) (break `/Game/Blueprints/Structs/SD_Playerinfo` (`self.PlayerInfo`)))
  (switch `/Game/Blueprints/Enums/E_MovementStates` (`self.MovementStates`)
    (:`NewEnumerator1`
      (`PaperFlipbookComponent.SetFlipbook` (`self.Sprite`) _idleanimation))
    (:`NewEnumerator2`
      (`SceneComponent.K2_AddRelativeRotation` :`self` (`self.Sprite`))
      (`KismetSystemLibrary.PrintString` "右边")
      (`PaperFlipbookComponent.SetFlipbook` (`self.Sprite`) _runanimation))
    (:`NewEnumerator3`
      (`SceneComponent.K2_AddRelativeRotation` (`self.Sprite`) (struct :`Yaw` 180.0) false false)
      (`KismetSystemLibrary.PrintString` "左边")
      (`PaperFlipbookComponent.SetFlipbook` (`self.Sprite`) _runanimation))
    (:`NewEnumerator4`
      (`PaperFlipbookComponent.SetFlipbook` (`self.Sprite`) _jumpanimation)
      (`GameplayStatics.PlaySound2D` "/Game/Assets/Audio/SFX_Jump.SFX_Jump" 1.0 1.0 0.0 null null))
    (:`NewEnumerator5`
      (`PaperFlipbookComponent.SetFlipbook` (`self.Sprite`) _fallanimation))))

(fn `UserConstructionScript`
  (`parent.UserConstructionScript`))