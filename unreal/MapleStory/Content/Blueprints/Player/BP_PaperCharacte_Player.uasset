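; Networked Paper2D player character with Enhanced Input for running, jumping, climbing and attacking.
; Input sets a movement state through server events, and its OnRep swaps flipbooks from CharacterPlayerInfo and flips the sprite.
; BeginPlay spawns a separate camera that timers and a timeline lerp toward the sampled player position, pausable by halting the sampling.
; Server events also set climb state, multicast jump sounds and fetch the game mode's spawn location, applied through OnRep.
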(event `UpdateCameraPosition`
  (bind _playercamera (`self.PlayerCamera`))
  ;[1 1 1] 相机跟随角色移动
  (bind (_direction _movementalpha) (`Timeline|PlayerCameraPostion` :!via `PlayFromStart`)
    (:`Update`
      (`/Engine/EditorBlueprintResources/StandardMacros.IsValid` _playercamera
        (:`Is Valid`
          (`self.K2_SetActorLocation` _playercamera (`KismetMathLibrary.VLerp` (`self.K2_GetActorLocation` (`self.PlayerCamera`)) (`self.CurrentPlayerLocation`) _movementalpha) false false))))))

(event `self.ReceiveBeginPlay`
  ;[1 1 1] 设置增强输入
  (message `EnhancedInputSubsystemInterface.AddMappingContext` (pcsubsystem `EnhancedInputLocalPlayerSubsystem` (`GameplayStatics.GetPlayerController` 0)) "/Game/Input/IMC_Default.IMC_Default" 0 (struct))
  (`self.SetPlayerSpawnLocation`)
  ;[1 1 1] 为角色动态生成摄像机
  (bind _returnvalue (`|SpawnActorFromClass` "/Game/Blueprints/BP_Camera.BP_Camera_C" (`KismetMathLibrary.MakeTransform` (`self.K2_GetActorLocation`)) "AdjustIfPossibleButAlwaysSpawn" "OverrideRootScale" null null))
  (`KismetSystemLibrary.Delay` 0.01)
  ;[1 1 1] 将视角切换给新的摄像机
  (set `self.PlayerCamera` _returnvalue)
  (bind _myplayercontroller (message `/Game/Blueprints/Interface/INT_PlayerController.GetMyPlayerController` (`self.GetController`)))
  (`/Engine/EditorBlueprintResources/StandardMacros.IsValid` _myplayercontroller
    (:`Is Valid`
      (`PlayerController.SetViewTargetWithBlend` _myplayercontroller (`self.PlayerCamera`) 0.0 "VTBlend_Linear" 0.0 false)
      ;[1 1 1] 相机跟随角色移动
      (bind _returnvalue_2 (`KismetSystemLibrary.K2_SetTimerDelegate` (delegate `UpdateCameraPosition`) 0.03 true))
      (set `self.UpdatePlayerCameraPositionHandle` _returnvalue_2)
      (bind _returnvalue_3 (`KismetSystemLibrary.K2_SetTimer` null "GetCurrentPlayerLocation" 0.1 true))
      (set `self.GetCurrentPlayerLocationHandle` _returnvalue_3))))

(event `self.PausePlayerCamera`
  (params (Pause :type Boolean))
  ;[1 1 1] 服务器端触发
  (`self.CL_PausePlayerCamera` Pause))

(event `EnhancedInput|/Game/Input/IA_Input/IA_MoveLeftRight`
  (params (ActionValue :type "Float (double-precision)") (ElapsedSeconds :type "Float (double-precision)") (TriggeredSeconds :type "Float (double-precision)") (InputAction :type "InputAction Object Reference" :default "/Game/Input/IA_Input/IA_MoveLeftRight.IA_MoveLeftRight"))
  ;[1 1 1] 移动并设置 移动状态
  (:`Triggered`
    (`self.AddMovementInput` (`KismetMathLibrary.GetForwardVector` (`self.GetControlRotation`)) ActionValue)
    (if (> ActionValue 0.0)
      (`self.SetMovementState` "NewEnumerator1")
      (else
        (`self.SetMovementState` "NewEnumerator2"))))
  (:`Completed`
    (`self.SetMovementState` "NewEnumerator0")))

(event `CL_PausePlayerCamera`
  (params (Pause :type Boolean))
  (bind _getcurrentplayerlocationhandle (`self.GetCurrentPlayerLocationHandle`))
  ;[1 1 1] 客户端本地暂停
  (if Pause
    (`KismetSystemLibrary.K2_PauseTimerHandle` _getcurrentplayerlocationhandle)
    (else
      (`KismetSystemLibrary.K2_UnPauseTimerHandle` _getcurrentplayerlocationhandle))))

(event `self.CanClamb`
  (params (CanClamb :type Boolean) (ClambingObject :type "PaperSpriteActor Object Reference"))
  (`self.SRV_CanClamb` CanClamb ClambingObject))

(event `EnhancedInput|/Game/Input/IA_Input/IA_MoveUpDown`
  (params (ActionValue :type "Float (double-precision)") (ElapsedSeconds :type "Float (double-precision)") (TriggeredSeconds :type "Float (double-precision)") (InputAction :type "InputAction Object Reference" :default "/Game/Input/IA_Input/IA_MoveUpDown.IA_MoveUpDown"))
  (bind _returnvalue (`KismetMathLibrary.GetUpVector` (`self.GetControlRotation`)))
  (:`Triggered`
    (if (`self.Can Clamb`)
      (`KismetSystemLibrary.PrintString` (`KismetStringLibrary.Conv_VectorToString` _returnvalue))
      (`self.AddMovementInput` _returnvalue ActionValue)
      (`self.SetMovementState` "NewEnumerator6"))))

(event `SRV_CanClamb`
  (params (CanClamb :type Boolean) (ClambingObject :type "PaperSpriteActor Object Reference"))
  (set `self.Can Clamb` CanClamb)
  (set `self.Clambing Object` ClambingObject))

(event `SetMovementState`
  (params (MovementState :type "/Game/Blueprints/Enums/E_MovementState Enum" :default "NewEnumerator0"))
  ;[1 1 1] 客户端函数
  (`self.SRV_SetMovementState` MovementState))

(event `SRV_SetMovementState`
  (params (MovementState :type "/Game/Blueprints/Enums/E_MovementState Enum" :default "NewEnumerator0"))
  ;[1 1 1] 服务端函数
  (set `self.MovementState` MovementState))

(event `EnhancedInput|/Game/Input/IA_Input/IA_Jump`
  (params (ActionValue :type Boolean) (ElapsedSeconds :type "Float (double-precision)") (TriggeredSeconds :type "Float (double-precision)") (InputAction :type "InputAction Object Reference" :default "/Game/Input/IA_Input/IA_Jump.IA_Jump"))
  ;[1 1 1] 跳跃
  (:`Triggered`
    (`self.Jump`)
    (`self.SetMovementState` "NewEnumerator3")
    (`KismetSystemLibrary.Delay` 0.5)
    (`self.SetMovementState` "NewEnumerator0"))
  (:`Started`
    (`self.SRV_Jump` (`.JumpSFX_14_8220B6DA4D38CB081513A8A1E6CEBCF3` (break `/Game/Blueprints/Structure/ST_PlayerInfo` (`self.CharacterPlayerInfo`))) (`self.K2_GetActorLocation`))))

(event `EnhancedInput|/Game/Input/IA_Input/IA_Attack`
  (params (ActionValue :type Boolean) (ElapsedSeconds :type "Float (double-precision)") (TriggeredSeconds :type "Float (double-precision)") (InputAction :type "InputAction Object Reference" :default "/Game/Input/IA_Input/IA_Attack.IA_Attack"))
  ;[1 1 1] 攻击
  (:`Triggered`
    (`self.SetMovementState` "NewEnumerator5")
    (`KismetSystemLibrary.Delay` 0.3)
    (`self.SetMovementState` "NewEnumerator0")))

(event `MC_Jump`
  (params (Sound :type "SoundBase Object Reference") (Location :type "Vector Structure"))
  ;[1 1 1] 播放声音
  (`GameplayStatics.PlaySoundAtLocation` Sound Location (struct) 1.0 1.0 0.0 null null null null))

(event `SRV_Jump`
  (params (Sound :type "SoundBase Object Reference") (Location :type "Vector Structure"))
  ;[1 1 1] 播放声音
  (`self.MC_Jump` Sound Location))

(event `self.SetPlayerSpawnLocation`
  ;[1 1 1] 设置玩家出生点
  (`self.SRV_SetPlayerSpawnLocation`))

(event `SRV_SetPlayerSpawnLocation`
  ;[1 1 1] 设置玩家出生点
  (bind _mygamemode (message `/Game/Blueprints/Interface/INT_GameMode.GetGameModeRef` (`GameplayStatics.GetGameMode`)))
  (set `self.Player Spawn Location` (`/Game/BP_MS_GameMode.PlayerSpawnLocation` _mygamemode)))

(fn `GetCurrentPlayerLocation`
  (set `self.CurrentPlayerLocation` (`self.K2_GetActorLocation`)))

(fn `GetPlayerRef`
  (returns (Player :type "/Game/Blueprints/Player/BP_PaperCharacte_Player Object Reference"))
  (return self))

(fn `OnRep_Can Clamb`)

(fn `OnRep_Clambing Object`)

(fn `OnRep_MovementState`
  (bind _sprite (`self.Sprite`))
  (bind _sprite_2 (`self.Sprite`))
  (bind (_idleanimation _runanimation _jumpanimation _attackanimation _fallanimation _jumpsfx _clambanimation) (break `/Game/Blueprints/Structure/ST_PlayerInfo` (`self.CharacterPlayerInfo`)))
  (switch `/Game/Blueprints/Enums/E_MovementState` (`self.MovementState`)
    (:`NewEnumerator0`
      (`PaperFlipbookComponent.SetFlipbook` _sprite _idleanimation))
    (:`NewEnumerator1`
      (`SceneComponent.K2_SetRelativeRotation` :`self` _sprite)
      (`PaperFlipbookComponent.SetFlipbook` _sprite_2 _runanimation))
    (:`NewEnumerator2`
      (`SceneComponent.K2_SetRelativeRotation` _sprite (struct :`Yaw` 180.0) false false)
      (`PaperFlipbookComponent.SetFlipbook` _sprite_2 _runanimation))
    (:`NewEnumerator3`
      (`PaperFlipbookComponent.SetFlipbook` _sprite _jumpanimation))
    (:`NewEnumerator4`
      (`PaperFlipbookComponent.SetFlipbook` _sprite _fallanimation))
    (:`NewEnumerator5`
      (`PaperFlipbookComponent.SetFlipbook` (`self.Sprite`) _attackanimation))
    (:`NewEnumerator6`
      (`PaperFlipbookComponent.SetFlipbook` (`self.Sprite`) _clambanimation))))

(fn `OnRep_Player Spawn Location`
  (`self.K2_SetActorLocation` (`self.Player Spawn Location`)))

(fn `UserConstructionScript`
  (`parent.UserConstructionScript`))