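; Behavior tree task that picks a random patrol-style destination for an enemy along the world X axis.
; It samples a reachable navmesh point around the pawn, with a radius spanning the first NavMeshBoundsVolume's full X width.
; Only that point's X is kept, combined with the pawn's current Y and Z, and written to the XLocationVector blackboard key.
; It then enables the enemy's movement state via a message call and finishes successfully.
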(event `self.ReceiveExecuteAI`
  (params (OwnerController :type "AIController Object Reference") (ControlledPawn :type "Pawn Object Reference"))
  (bind _enemy (message `/Game/Blueprints/Interface/INT_EnemyBase.GetEnemyRef` ControlledPawn))
  (set `self.EnemyPawn` _enemy)
  (bind _outactors (`GameplayStatics.GetAllActorsOfClass` "/Script/NavigationSystem.NavMeshBoundsVolume"))
  (`BTFunctionLibrary.SetBlackboardValueAsVector` (`self.XLocationVector`) (`KismetMathLibrary.MakeVector` (.x (`NavigationSystemV1.K2_GetRandomReachablePointInRadius` (`Actor.K2_GetActorLocation` (`self.EnemyPawn`)) (* (.x (`.BoxExtent` (`Actor.GetActorBounds` (`|GetArrayItem` _outactors) false false))) 2.0) null null)) (.y (`Actor.K2_GetActorLocation` (`self.EnemyPawn`))) (.z (`Actor.K2_GetActorLocation` (`self.EnemyPawn`)))))
  (message `/Game/Blueprints/Interface/INT_EnemyBase.SetMovementState` (`self.EnemyPawn`) true)
  (`self.FinishExecute` true))