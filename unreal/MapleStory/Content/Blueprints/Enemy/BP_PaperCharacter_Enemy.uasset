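; Enemy Paper2D character Blueprint that keeps its sprite animation in step with a replicated movement state.
; SetMovementState forwards to SRV_SetMovementState, named as a server event, which sets IsMoving.
; OnRep_IsMoving then switches the sprite between the move and idle flipbooks from AnimationInfo.
; GetEnemyRef returns the enemy itself, and the default BeginPlay, overlap and Tick events are unused.
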(event `SRV_SetMovementState`
  (params (IsMoving :type Boolean))
  (set `self.IsMoving` IsMoving))

(event `/Game/Blueprints/Interface/INT_EnemyBase.SetMovementState`
  (params (IsMoving :type Boolean))
  (`self.SRV_SetMovementState` IsMoving))

(fn `GetEnemyRef`
  (returns (Enemy :type "/Game/Blueprints/Enemy/BP_PaperCharacter_Enemy Object Reference"))
  (return self))

(fn `OnRep_IsMoving`
  (bind _sprite (`self.Sprite`))
  (bind (_idleanimation _moveanimation) (break `/Game/Blueprints/Structure/ST_EnemyInfo` (`self.AnimationInfo`)))
  (if (`self.IsMoving`)
    (`PaperFlipbookComponent.SetFlipbook` _sprite _moveanimation)
    (else
      (`PaperFlipbookComponent.SetFlipbook` _sprite _idleanimation))))

(fn `UserConstructionScript`
  (`parent.UserConstructionScript`))