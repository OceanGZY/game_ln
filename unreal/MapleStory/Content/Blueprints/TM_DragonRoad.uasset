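; TM_DragonRoad is a road actor with left and right trigger boxes that pause the player's camera while a player is inside either one.
; On the server only, overlaps with actors tagged "Player" send interface-style messages: pause camera on entering, resume on leaving.
; Each box acts independently with no overlap count, so leaving one box resumes the camera even if the player remains in the other.
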(event `self.LeftBox.OnComponentBeginOverlap`
  (params (OverlappedComponent :type "PrimitiveComponent Object Reference") (OtherActor :type "Actor Object Reference") (OtherComp :type "PrimitiveComponent Object Reference") (OtherBodyIndex :type Integer) (bFromSweep :type Boolean) (SweepResult :type "HitResult Structure (by ref)"))
  ;[1 1 1] 判断当前对象是否是本地对象, remote为客户端
  (`/Engine/EditorBlueprintResources/ActorMacros.Switch Has Authority`
    (:`Authority`
      (if (`self.ActorHasTag` OtherActor "Player")
        (message `/Game/Blueprints/Interface/INT_PlayerBase.GetPlayerRef` OtherActor)
        (message `/Game/Blueprints/Interface/INT_PlayerBase.PausePlayerCamera` OtherActor true)))))

(event `self.LeftBox.OnComponentEndOverlap`
  (params (OverlappedComponent :type "PrimitiveComponent Object Reference") (OtherActor :type "Actor Object Reference") (OtherComp :type "PrimitiveComponent Object Reference") (OtherBodyIndex :type Integer))
  ;[1 1 1] 判断当前对象是否是本地对象, remote为客户端
  (`/Engine/EditorBlueprintResources/ActorMacros.Switch Has Authority`
    (:`Authority`
      (if (`self.ActorHasTag` OtherActor "Player")
        (message `/Game/Blueprints/Interface/INT_PlayerBase.GetPlayerRef` OtherActor)
        (message `/Game/Blueprints/Interface/INT_PlayerBase.PausePlayerCamera` OtherActor false)))))

(event `self.RightBox.OnComponentBeginOverlap`
  (params (OverlappedComponent :type "PrimitiveComponent Object Reference") (OtherActor :type "Actor Object Reference") (OtherComp :type "PrimitiveComponent Object Reference") (OtherBodyIndex :type Integer) (bFromSweep :type Boolean) (SweepResult :type "HitResult Structure (by ref)"))
  ;[1 1 1] 判断当前对象是否是本地对象, remote为客户端
  (`/Engine/EditorBlueprintResources/ActorMacros.Switch Has Authority`
    (:`Authority`
      (if (`self.ActorHasTag` OtherActor "Player")
        (message `/Game/Blueprints/Interface/INT_PlayerBase.GetPlayerRef` OtherActor)
        (message `/Game/Blueprints/Interface/INT_PlayerBase.PausePlayerCamera` OtherActor true)))))

(event `self.RightBox.OnComponentEndOverlap`
  (params (OverlappedComponent :type "PrimitiveComponent Object Reference") (OtherActor :type "Actor Object Reference") (OtherComp :type "PrimitiveComponent Object Reference") (OtherBodyIndex :type Integer))
  ;[1 1 1] 判断当前对象是否是本地对象, remote为客户端
  (`/Engine/EditorBlueprintResources/ActorMacros.Switch Has Authority`
    (:`Authority`
      (if (`self.ActorHasTag` OtherActor "Player")
        (message `/Game/Blueprints/Interface/INT_PlayerBase.GetPlayerRef` OtherActor)
        (message `/Game/Blueprints/Interface/INT_PlayerBase.PausePlayerCamera` OtherActor false)))))

(fn `UserConstructionScript`)