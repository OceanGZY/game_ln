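; BP_MS_GameController is a player controller that handles character selection and spawning.
; On BeginPlay, a client event creates the WB_ChooseCharacter widget and adds it to the viewport.
; SelectCharacter forwards the chosen class and location to a server event, which requests a spawn from the game mode via a message call.
; SpawnPlayer spawns that class, adjusting for collisions but always spawning, then possesses it.
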(event `self.ReceiveBeginPlay`
  (`self.InitializeWidgets`))

(event `self.InitializeWidgets`
  (`self.CL_InitializWidgets`))

(event `CL_InitializWidgets`
  (bind _returnvalue (`|CreateWidget` "/Game/UI/HUD/WB_ChooseCharacter.WB_ChooseCharacter_C"))
  (bind _output_get (set `self.WB_ChooseCharacter` _returnvalue))
  (`/Engine/EditorBlueprintResources/StandardMacros.IsValid` _output_get
    (:`Is Valid`
      (`UserWidget.AddToViewport` _output_get 0))))

(event `self.SelectCharacter`
  (params (Player :type "Actor Class Reference") (SpawnLocation :type "Vector Structure"))
  ;[1 1 1] 客户端 触发选角色，通知服务器
  (`self.SRV_SelectCharacter` Player SpawnLocation))

(event `SRV_SelectCharacter`
  (params (Player :type "Actor Class Reference") (SpwanLocation :type "Vector Structure"))
  ;[1 1 1] 服务器查游戏模式，允许的话，则生成角色
  (bind _mygamemode (message `/Game/Blueprints/Interface/INT_GameMode.GetGameModeRef` (`GameplayStatics.GetGameMode`)))
  (message `/Game/Blueprints/Interface/INT_GameMode.RequestSpwanPlayer` _mygamemode self Player SpwanLocation))

(event `self.SpawnPlayer`
  (params (Player :type "Actor Class Reference") (SpawnTransform :type "Transform Structure"))
  ;[1 1 1] 生成角色
  (bind _returnvalue (`|SpawnActorFromClass` Player SpawnTransform "AdjustIfPossibleButAlwaysSpawn" "OverrideRootScale" null null))
  (bind _player (message `/Game/Blueprints/Interface/INT_PlayerBase.GetPlayerRef` _returnvalue))
  (`self.Possess` _player))

(fn `GetMyPlayerController`
  (returns (MyPlayerController :type "/Game/BP_MS_GameController Object Reference"))
  (return self))

(fn `UserConstructionScript`)